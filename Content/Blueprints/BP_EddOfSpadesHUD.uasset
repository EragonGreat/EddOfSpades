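; BP_EddOfSpadesHUD is the game's HUD Blueprint, which creates and controls the main on-screen UI.
; On BeginPlay it creates a UI_Main widget for the first player controller, adds it to the viewport and stores it as MainWidget.
; ToggleColorPalette shows or hides that widget's color wheel.
; ProgressItemCountChanged clears the widget's progress list and rebuilds it from the keys of the ProgressItems map.
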(event Custom|ToggleColorPalette
  (params (Visible :type Boolean))
  (bind _mainwidget (Variables|Default|GetMainWidget))
  (bind _colorwheelcontainer (Variables|/Game/Widgets/UI_Main.UI_Main_C|GetColorWheelContainer _mainwidget))
  (if Visible
    (Widget|SetVisibility _colorwheelcontainer "Visible")
    (else
      (Widget|SetVisibility _colorwheelcontainer "Hidden"))))

(event EventBeginPlay
  (bind _returnvalue (UserInterface|CreateWidget "/Game/Widgets/UI_Main.UI_Main_C" (Game|GetPlayerController 0)))
  (UserInterface|Viewport|AddtoViewport _returnvalue 0)
  (Variables|Default|SetMainWidget _returnvalue))

(event Collision|EventActorBeginOverlap
  (params (OtherActor :type Actor%20Object%20Reference)))

(event EventTick
  (params (DeltaSeconds :type Float%20%28single-precision%29)))

(event EventProgressItemCountChanged
  (Default|ClearAllItems (Variables|/Game/Widgets/UI_Main.UI_Main_C|GetUI_ProgressItemList (Variables|Default|GetMainWidget)))
  (bind _keys (Utilities|Map|Keys (Variables|Default|GetProgressItems)))
  (for _array_element _keys
    (Default|AddProgressItem (Variables|/Game/Widgets/UI_Main.UI_Main_C|GetUI_ProgressItemList (Variables|Default|GetMainWidget)) _array_element)))

(fn ConstructionScript)