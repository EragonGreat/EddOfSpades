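; Player controller for Edd of Spades that handles toggling the HUD color palette and the mouse cursor.
; The palette input drives the palette on BP_EddOfSpadesHUD and switches input mode along with it, while a separate input toggles only the cursor.
; SetRealInputMode swaps between Game and UI with a visible, locked cursor and Game Only with it hidden.
; Each input keeps its own FlipFlop state, independent of the other.
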(event EventTick
  (params (DeltaSeconds :type Float%20%28single-precision%29)))

(event Input|ActionEvents|InputActionToggleCursor
  (params (Key :type Key%20Structure))
  (:Pressed
    (bind _isa (Utilities|FlowControl|FlipFlop)
      (:A
        _)
      (:B
        _))
    (CallFunction|SetRealInputMode _isa)))

(event Input|ActionEvents|InputActionToggleColorPalette
  (params (Key :type Key%20Structure))
  (:Pressed
    (bind _isa (Utilities|FlowControl|FlipFlop)
      (:A
        _)
      (:B
        _))
    (Default|ToggleColorPalette (.AsBP%20Edd%20Of%20Spades%20HUD (Utilities|Casting|CastToBP_EddOfSpadesHUD (HUD|GetHUD))) _isa)
    (CallFunction|SetRealInputMode _isa)))

(event Input|ActionEvents|InputActionToggleFPSCounter
  (params (Key :type Key%20Structure)))

(fn ConstructionScript)

(fn SetRealInputMode
  (params (ShowCursor :type Boolean))
  (if ShowCursor
    (Input|SetInputModeGameandUI self 0 "LockAlways" false)
    (Variables|Default|SetbShowMouseCursor true)
    (else
      (Variables|Default|SetbShowMouseCursor false)
      (Input|SetInputModeGameOnly self))))